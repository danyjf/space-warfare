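; Orbit camera pawn that follows a focused actor, starting on the first CPP_Planet found at BeginPlay.
; Tick snaps the pawn to that actor's location, while mouse axes add controller yaw and inverted pitch.
; A short left click, timed against a threshold, traces under the cursor and refocuses on any actor with a BP_CameraOrbitableComponent.
; That component supplies the spring arm's orbit distance and the mouse wheel's zoom step and limits.
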(event EventBeginPlay
  (bind _returnvalue (Actor|GetActorOfClass "/Script/SpaceWarfare.CPP_Planet"))
  (bind _output_get (Variables|Default|SetOrbitingActor _returnvalue))
  (Transformation|SetActorLocation (Transformation|GetActorLocation _output_get) false false)
  (Variables|Default|SetCameraOrbitableComponent (Actor|GetComponentbyClass _output_get "/Game/SpaceWarfare/Core/CameraControls/BP_CameraOrbitableComponent.BP_CameraOrbitableComponent_C")))

(event EventTick
  (params (DeltaSeconds :type Float%20%28single-precision%29))
  (Variables|Default|SetClickTimer (+ DeltaSeconds (Variables|Default|GetClickTimer)))
  (Transformation|SetActorLocation (Transformation|GetActorLocation (Variables|Default|GetOrbitingActor)) false false))

(event Input|MouseEvents|MouseX
  (params (AxisValue :type Float%20%28single-precision%29))
  (Pawn|Input|AddControllerYawInput AxisValue))

(event Input|MouseEvents|MouseY
  (params (AxisValue :type Float%20%28single-precision%29))
  (Pawn|Input|AddControllerPitchInput (* AxisValue -1.0)))

(event Input|MouseEvents|LeftMouseButton
  (params (Key :type Key%20Structure :default "None"))
  (bind _returnvalue (Game|GetPlayerState 0))
  (bind _returnvalue_2 (Game|GetPlayerController _returnvalue))
  (bind _hitresult (Game|Player|GetHitResultUnderCursorbyChannel _returnvalue_2 "TraceTypeQuery1" true))
  (bind _hitactor (Collision|BreakHitResult _hitresult))
  (bind _returnvalue_3 (Actor|GetComponentbyClass _hitactor "/Game/SpaceWarfare/Core/CameraControls/BP_CameraOrbitableComponent.BP_CameraOrbitableComponent_C"))
  (:Pressed
    (Variables|Default|SetClickTimer 0.0))
  (:Released
    (if (<= (Variables|Default|GetClickTimer) (Variables|Default|GetClickThreshold))
      (Utilities|IsValid _hitactor
        (:Is%20Valid
          (Utilities|IsValid _returnvalue_3
            (:Is%20Valid
              (Variables|Default|SetCameraOrbitableComponent _returnvalue_3)
              (Variables|/Script/Engine.SpringArmComponent|SetTargetArmLength (Variables|Default|GetSpringArm) (Variables|/Game/SpaceWarfare/Core/CameraControls/BP_CameraOrbitableComponent.BP_CameraOrbitableComponent_C|GetOrbitDistance (Variables|Default|GetCameraOrbitableComponent)))
              (Variables|Default|SetOrbitingActor _hitactor))))))))

(event Input|MouseEvents|MouseWheelUp
  (params (Key :type Key%20Structure :default "None"))
  (bind _springarm (Variables|Default|GetSpringArm))
  (bind _cameraorbitablecomponent (Variables|Default|GetCameraOrbitableComponent))
  (:Pressed
    (if (>= (- (Variables|/Script/Engine.SpringArmComponent|GetTargetArmLength _springarm) (Variables|/Game/SpaceWarfare/Core/CameraControls/BP_CameraOrbitableComponent.BP_CameraOrbitableComponent_C|GetZoomSpeed _cameraorbitablecomponent)) (Variables|/Game/SpaceWarfare/Core/CameraControls/BP_CameraOrbitableComponent.BP_CameraOrbitableComponent_C|GetMinOrbitDistance _cameraorbitablecomponent))
      (if (<= (- (Variables|/Script/Engine.SpringArmComponent|GetTargetArmLength _springarm) (Variables|/Game/SpaceWarfare/Core/CameraControls/BP_CameraOrbitableComponent.BP_CameraOrbitableComponent_C|GetZoomSpeed _cameraorbitablecomponent)) (Variables|/Game/SpaceWarfare/Core/CameraControls/BP_CameraOrbitableComponent.BP_CameraOrbitableComponent_C|GetMaxOrbitDistance _cameraorbitablecomponent))
        (Variables|/Script/Engine.SpringArmComponent|SetTargetArmLength _springarm (- (Variables|/Script/Engine.SpringArmComponent|GetTargetArmLength _springarm) (Variables|/Game/SpaceWarfare/Core/CameraControls/BP_CameraOrbitableComponent.BP_CameraOrbitableComponent_C|GetZoomSpeed _cameraorbitablecomponent)))))))

(event Input|MouseEvents|MouseWheelDown
  (params (Key :type Key%20Structure :default "None"))
  (bind _cameraorbitablecomponent (Variables|Default|GetCameraOrbitableComponent))
  (bind _springarm (Variables|Default|GetSpringArm))
  (:Pressed
    (if (>= (+ (Variables|/Script/Engine.SpringArmComponent|GetTargetArmLength _springarm) (Variables|/Game/SpaceWarfare/Core/CameraControls/BP_CameraOrbitableComponent.BP_CameraOrbitableComponent_C|GetZoomSpeed _cameraorbitablecomponent)) (Variables|/Game/SpaceWarfare/Core/CameraControls/BP_CameraOrbitableComponent.BP_CameraOrbitableComponent_C|GetMinOrbitDistance _cameraorbitablecomponent))
      (if (<= (+ (Variables|/Script/Engine.SpringArmComponent|GetTargetArmLength _springarm) (Variables|/Game/SpaceWarfare/Core/CameraControls/BP_CameraOrbitableComponent.BP_CameraOrbitableComponent_C|GetZoomSpeed _cameraorbitablecomponent)) (Variables|/Game/SpaceWarfare/Core/CameraControls/BP_CameraOrbitableComponent.BP_CameraOrbitableComponent_C|GetMaxOrbitDistance _cameraorbitablecomponent))
        (Variables|/Script/Engine.SpringArmComponent|SetTargetArmLength _springarm (+ (Variables|/Script/Engine.SpringArmComponent|GetTargetArmLength _springarm) (Variables|/Game/SpaceWarfare/Core/CameraControls/BP_CameraOrbitableComponent.BP_CameraOrbitableComponent_C|GetZoomSpeed _cameraorbitablecomponent)))))))

(fn ConstructionScript)