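; Camera orbit controller for SpaceWarfare that rotates and zooms the player's view, starting in God Mode input.
; In God Mode, mouse axes drive pawn yaw and inverted pitch; in Ground Station mode, render-target drag events drive both, scaled by drag speed.
; The wheel steps spring arm length within the orbitable component's limits, requiring render-target hover in Ground Station mode.
; Left mouse press and release are forwarded to handler functions.
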(event Custom|OnMouseDragTargetRender
  (params (MouseDeltaX :type Float%20%28double-precision%29) (MouseDeltaY :type Float%20%28double-precision%29))
  (bind _rendertargetdragspeed (Variables|Default|GetRenderTargetDragSpeed))
  (bind _playerpawn (Variables|Default|GetPlayerPawn))
  (switch Utilities|FlowControl|Switch|SwitchonEInputMode (Variables|Default|GetInputMode)
    (:GROUNDSTATIONINPUT
      (Pawn|Input|AddControllerYawInput _playerpawn (* MouseDeltaX _rendertargetdragspeed))
      (Pawn|Input|AddControllerPitchInput _playerpawn (* MouseDeltaY _rendertargetdragspeed)))))

(event EventBeginPlay
  (Variables|Default|SetInputMode "GODMODEINPUT"))

(event EventTick
  (params (DeltaSeconds :type Float%20%28single-precision%29)))

(event Input|MouseEvents|MouseX
  (params (AxisValue :type Float%20%28single-precision%29))
  (switch Utilities|FlowControl|Switch|SwitchonEInputMode (Variables|Default|GetInputMode)
    (:GODMODEINPUT
      (Pawn|Input|AddControllerYawInput (Variables|Default|GetPlayerPawn) AxisValue))))

(event Input|MouseEvents|MouseY
  (params (AxisValue :type Float%20%28single-precision%29))
  (switch Utilities|FlowControl|Switch|SwitchonEInputMode (Variables|Default|GetInputMode)
    (:GODMODEINPUT
      (Pawn|Input|AddControllerPitchInput (Variables|Default|GetPlayerPawn) (* AxisValue -1.0)))))

(event Input|MouseEvents|LeftMouseButton
  (params (Key :type Key%20Structure :default "None"))
  (:Pressed
    (Class|CPPCameraOrbitController|HandleLeftMouseButtonPress))
  (:Released
    (Class|CPPCameraOrbitController|HandleLeftMouseButtonRelease)))

(event Input|MouseEvents|MouseWheelUp
  (params (Key :type Key%20Structure :default "None"))
  (bind _cameraorbitablecomponent (Variables|Default|GetCameraOrbitableComponent))
  (bind _springarmcomponent (Variables|Default|GetSpringArmComponent))
  (:Pressed
    (switch Utilities|FlowControl|Switch|SwitchonEInputMode (Variables|Default|GetInputMode)
      (:GROUNDSTATIONINPUT
        (if (Variables|Default|GetIsHoveringRenderTarget)
          (if (>= (- (Variables|/Script/Engine.SpringArmComponent|GetTargetArmLength _springarmcomponent) (Variables|/Script/SpaceWarfare.CPP_CameraOrbitableComponent|GetZoomSpeed _cameraorbitablecomponent)) (Variables|/Script/SpaceWarfare.CPP_CameraOrbitableComponent|GetMinOrbitDistance _cameraorbitablecomponent)) :!label _label
            (if (<= (- (Variables|/Script/Engine.SpringArmComponent|GetTargetArmLength _springarmcomponent) (Variables|/Script/SpaceWarfare.CPP_CameraOrbitableComponent|GetZoomSpeed _cameraorbitablecomponent)) (Variables|/Script/SpaceWarfare.CPP_CameraOrbitableComponent|GetMaxOrbitDistance _cameraorbitablecomponent))
              (Variables|/Script/Engine.SpringArmComponent|SetTargetArmLength _springarmcomponent (- (Variables|/Script/Engine.SpringArmComponent|GetTargetArmLength _springarmcomponent) (Variables|/Script/SpaceWarfare.CPP_CameraOrbitableComponent|GetZoomSpeed _cameraorbitablecomponent)))))))
      (:GODMODEINPUT
        (goto _label)))))

(event Input|MouseEvents|MouseWheelDown
  (params (Key :type Key%20Structure :default "None"))
  (bind _cameraorbitablecomponent (Variables|Default|GetCameraOrbitableComponent))
  (bind _springarmcomponent (Variables|Default|GetSpringArmComponent))
  (:Pressed
    (switch Utilities|FlowControl|Switch|SwitchonEInputMode (Variables|Default|GetInputMode)
      (:GROUNDSTATIONINPUT
        (if (Variables|Default|GetIsHoveringRenderTarget)
          (if (>= (+ (Variables|/Script/Engine.SpringArmComponent|GetTargetArmLength _springarmcomponent) (Variables|/Script/SpaceWarfare.CPP_CameraOrbitableComponent|GetZoomSpeed _cameraorbitablecomponent)) (Variables|/Script/SpaceWarfare.CPP_CameraOrbitableComponent|GetMinOrbitDistance _cameraorbitablecomponent)) :!label _label
            (if (<= (+ (Variables|/Script/Engine.SpringArmComponent|GetTargetArmLength _springarmcomponent) (Variables|/Script/SpaceWarfare.CPP_CameraOrbitableComponent|GetZoomSpeed _cameraorbitablecomponent)) (Variables|/Script/SpaceWarfare.CPP_CameraOrbitableComponent|GetMaxOrbitDistance _cameraorbitablecomponent))
              (Variables|/Script/Engine.SpringArmComponent|SetTargetArmLength _springarmcomponent (+ (Variables|/Script/Engine.SpringArmComponent|GetTargetArmLength _springarmcomponent) (Variables|/Script/SpaceWarfare.CPP_CameraOrbitableComponent|GetZoomSpeed _cameraorbitablecomponent)))))))
      (:GODMODEINPUT
        (goto _label)))))

(fn ConstructionScript)