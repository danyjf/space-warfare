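; Player controller for SpaceWarfare that handles zoom and drag rotation of an orbit camera.
; Mouse wheel steps the spring arm length by the orbitable component's zoom speed, skipping any step that would leave its min and max orbit distances.
; A render-target mouse drag event feeds scaled mouse deltas into the player pawn's controller yaw and pitch input.
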(event Custom|OnMouseDragTargetRender
  (params (MouseDeltaX :type Float%20%28double-precision%29) (MouseDeltaY :type Float%20%28double-precision%29))
  (bind _rendertargetdragspeed (Variables|Default|GetRenderTargetDragSpeed))
  (bind _playerpawn (Variables|Default|GetPlayerPawn))
  (Pawn|Input|AddControllerYawInput _playerpawn (* MouseDeltaX _rendertargetdragspeed))
  (Pawn|Input|AddControllerPitchInput _playerpawn (* MouseDeltaY _rendertargetdragspeed)))

(event EventBeginPlay)

(event EventTick
  (params (DeltaSeconds :type Float%20%28single-precision%29)))

(event Input|MouseEvents|MouseWheelUp
  (params (Key :type Key%20Structure :default "None"))
  (bind _cameraorbitablecomponent (Variables|Default|GetCameraOrbitableComponent))
  (bind _springarmcomponent (Variables|Default|GetSpringArmComponent))
  (:Pressed
    (if (>= (- (Variables|/Script/Engine.SpringArmComponent|GetTargetArmLength _springarmcomponent) (Variables|/Script/SpaceWarfare.CPP_CameraOrbitableComponent|GetZoomSpeed _cameraorbitablecomponent)) (Variables|/Script/SpaceWarfare.CPP_CameraOrbitableComponent|GetMinOrbitDistance _cameraorbitablecomponent))
      (if (<= (- (Variables|/Script/Engine.SpringArmComponent|GetTargetArmLength _springarmcomponent) (Variables|/Script/SpaceWarfare.CPP_CameraOrbitableComponent|GetZoomSpeed _cameraorbitablecomponent)) (Variables|/Script/SpaceWarfare.CPP_CameraOrbitableComponent|GetMaxOrbitDistance _cameraorbitablecomponent))
        (Variables|/Script/Engine.SpringArmComponent|SetTargetArmLength _springarmcomponent (- (Variables|/Script/Engine.SpringArmComponent|GetTargetArmLength _springarmcomponent) (Variables|/Script/SpaceWarfare.CPP_CameraOrbitableComponent|GetZoomSpeed _cameraorbitablecomponent)))))))

(event Input|MouseEvents|MouseWheelDown
  (params (Key :type Key%20Structure :default "None"))
  (bind _cameraorbitablecomponent (Variables|Default|GetCameraOrbitableComponent))
  (bind _springarmcomponent (Variables|Default|GetSpringArmComponent))
  (:Pressed
    (if (>= (+ (Variables|/Script/Engine.SpringArmComponent|GetTargetArmLength _springarmcomponent) (Variables|/Script/SpaceWarfare.CPP_CameraOrbitableComponent|GetZoomSpeed _cameraorbitablecomponent)) (Variables|/Script/SpaceWarfare.CPP_CameraOrbitableComponent|GetMinOrbitDistance _cameraorbitablecomponent))
      (if (<= (+ (Variables|/Script/Engine.SpringArmComponent|GetTargetArmLength _springarmcomponent) (Variables|/Script/SpaceWarfare.CPP_CameraOrbitableComponent|GetZoomSpeed _cameraorbitablecomponent)) (Variables|/Script/SpaceWarfare.CPP_CameraOrbitableComponent|GetMaxOrbitDistance _cameraorbitablecomponent))
        (Variables|/Script/Engine.SpringArmComponent|SetTargetArmLength _springarmcomponent (+ (Variables|/Script/Engine.SpringArmComponent|GetTargetArmLength _springarmcomponent) (Variables|/Script/SpaceWarfare.CPP_CameraOrbitableComponent|GetZoomSpeed _cameraorbitablecomponent)))))))

(fn ConstructionScript)