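; BP_BotGameHUD is the HUD for the bot game mode, setting up the player's on-screen UI at BeginPlay.
; It creates WBP_GameScreen, resets its widget switcher to the first page and adds it to the viewport.
; If the game instance's max session player count is nonzero, it also shows a WBP_WaitForPlayers overlay.
; It then shows the mouse cursor and sets Game and UI input mode.
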(event EventBeginPlay
  (bind _returnvalue (Game|GetPlayerController 0))
  (bind _returnvalue_2 (UserInterface|CreateWidget "/Game/SpaceWarfare/UI/Game/WBP_GameScreen.WBP_GameScreen_C"))
  (bind _output_get (Variables|Default|SetGameScreenWidget _returnvalue_2))
  (bind _aswbp_game_screen (Utilities|Casting|CastToWBP_GameScreen _output_get))
  (bind _output_get_2 (Variables|Default|SetWBP_GameScreen _aswbp_game_screen))
  (Class|WidgetSwitcher|SetActiveWidgetIndex (Variables|/Game/SpaceWarfare/UI/Game/WBP_GameScreen.WBP_GameScreen_C|GetWidgetSwitcher _output_get_2))
  (UserInterface|Viewport|AddtoViewport _output_get_2 0)
  (bind _asbp_game_instance (Utilities|Casting|CastToBP_GameInstance (Game|GetGameInstance)))
  (if (== (Variables|/Script/SpaceWarfare.CPP_GameInstance|GetMaxNumberOfPlayersInSession _asbp_game_instance) 0)
    _
    (else
      (bind _returnvalue_3 (UserInterface|CreateWidget "/Game/SpaceWarfare/UI/Game/WBP_WaitForPlayers.WBP_WaitForPlayers_C"))
      (UserInterface|Viewport|AddtoViewport _returnvalue_3 0)))
  (Variables|/Script/Engine.PlayerController|SetbShowMouseCursor _returnvalue true)
  (Input|SetInputModeGameandUI _returnvalue 0 "DoNotLock" false false))

(event Collision|EventActorBeginOverlap
  (params (OtherActor :type Actor%20Object%20Reference)))

(event EventTick
  (params (DeltaSeconds :type Float%20%28single-precision%29)))

(fn ConstructionScript)