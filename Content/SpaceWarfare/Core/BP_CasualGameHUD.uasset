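; BP_CasualGameHUD builds the game screen for casual mode, a stripped-down variant of the satellite game UI.
; On BeginPlay it creates WBP_GameScreen on the SatelliteView, removing the ground stations view toggle, satellite command widgets and target checkbox.
; It adds a wait-for-players overlay when the GameInstance's session player maximum is nonzero, then shows the cursor and sets Game and UI input.
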(event EventBeginPlay
  (bind _returnvalue (Game|GetPlayerController 0))
  ;[1 1 1] Create the GameScreen and set the active widget to be the SatelliteView
  (bind _returnvalue_2 (UserInterface|CreateWidget "/Game/SpaceWarfare/UI/Game/WBP_GameScreen.WBP_GameScreen_C"))
  (bind _output_get (Variables|Default|SetGameScreenWidget _returnvalue_2))
  (bind _aswbp_game_screen (Utilities|Casting|CastToWBP_GameScreen _output_get))
  (bind _output_get_2 (Variables|Default|SetWBP_GameScreen _aswbp_game_screen))
  (Class|WidgetSwitcher|SetActiveWidgetIndex (Variables|/Game/SpaceWarfare/UI/Game/WBP_GameScreen.WBP_GameScreen_C|GetWidgetSwitcher _output_get_2))
  ;[1 1 1] Remove checkbox to go to the GroundStationsView screen
  (Widget|RemovefromParent (Variables|/Game/SpaceWarfare/UI/Game/WBP_GameScreen.WBP_GameScreen_C|GetGroundStationsViewSizeBox (Variables|Default|GetWBP_GameScreen)))
  ;[1 1 1] Remove commands UI
  (Widget|RemovefromParent (Variables|/Game/SpaceWarfare/UI/Game/SatelliteView/WBP_SatelliteInfo.WBP_SatelliteInfo_C|GetCommandsText (Variables|/Game/SpaceWarfare/UI/Game/SatelliteView/WBP_SatelliteView.WBP_SatelliteView_C|GetWBP_SatelliteInfo (Variables|/Game/SpaceWarfare/UI/Game/WBP_GameScreen.WBP_GameScreen_C|GetWBP_SatelliteView (Variables|Default|GetWBP_GameScreen)))))
  (Widget|RemovefromParent (Variables|/Game/SpaceWarfare/UI/Game/SatelliteView/WBP_SatelliteInfo.WBP_SatelliteInfo_C|GetNoCommandsText (Variables|/Game/SpaceWarfare/UI/Game/SatelliteView/WBP_SatelliteView.WBP_SatelliteView_C|GetWBP_SatelliteInfo (Variables|/Game/SpaceWarfare/UI/Game/WBP_GameScreen.WBP_GameScreen_C|GetWBP_SatelliteView (Variables|Default|GetWBP_GameScreen)))))
  (Widget|RemovefromParent (Variables|/Game/SpaceWarfare/UI/Game/SatelliteView/WBP_SatelliteInfo.WBP_SatelliteInfo_C|GetCommandsScrollBox (Variables|/Game/SpaceWarfare/UI/Game/SatelliteView/WBP_SatelliteView.WBP_SatelliteView_C|GetWBP_SatelliteInfo (Variables|/Game/SpaceWarfare/UI/Game/WBP_GameScreen.WBP_GameScreen_C|GetWBP_SatelliteView (Variables|Default|GetWBP_GameScreen)))))
  (Widget|RemovefromParent (Variables|/Game/SpaceWarfare/UI/Game/SatelliteView/WBP_SatelliteInfo.WBP_SatelliteInfo_C|GetTargetCheckBox (Variables|/Game/SpaceWarfare/UI/Game/SatelliteView/WBP_SatelliteView.WBP_SatelliteView_C|GetWBP_SatelliteInfo (Variables|/Game/SpaceWarfare/UI/Game/WBP_GameScreen.WBP_GameScreen_C|GetWBP_SatelliteView (Variables|Default|GetWBP_GameScreen)))))
  (UserInterface|Viewport|AddtoViewport (Variables|Default|GetWBP_GameScreen) 0)
  ;[1 1 1] Handle the screen with the wait for all players
  (bind _asbp_game_instance (Utilities|Casting|CastToBP_GameInstance (Game|GetGameInstance)))
  (if (== (Variables|/Script/SpaceWarfare.CPP_GameInstance|GetMaxNumberOfPlayersInSession _asbp_game_instance) 0)
    _
    (else
      (bind _returnvalue_3 (UserInterface|CreateWidget "/Game/SpaceWarfare/UI/Game/WBP_WaitForPlayers.WBP_WaitForPlayers_C"))
      (UserInterface|Viewport|AddtoViewport _returnvalue_3 0)))
  (Variables|/Script/Engine.PlayerController|SetbShowMouseCursor _returnvalue true)
  (Input|SetInputModeGameandUI _returnvalue 0 "DoNotLock" false false))

(event Collision|EventActorBeginOverlap
  (params (OtherActor :type Actor%20Object%20Reference)))

(event EventTick
  (params (DeltaSeconds :type Float%20%28single-precision%29)))

(fn ConstructionScript)